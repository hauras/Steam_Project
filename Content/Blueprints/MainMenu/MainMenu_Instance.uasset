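; MainMenu_Instance is a main menu Blueprint, apparently the game instance, that hosts multiplayer sessions.
; CreateServer creates an Advanced Sessions session from the given connection count and LAN flag, storing server name, language and LAN use as extra settings.
; On success it opens DevMap as a listen server; failure is not handled.
; GetGameInstanceRef returns the instance itself.
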(event `CreateServer`
  (params (ServerName :type String) (PublicConnections :type Integer) (bUseLAN :type Boolean) (Language :type String))
  (`CreateSessionCallbackProxyAdvanced.CreateAdvancedSession` (`|MakeArray` (`AdvancedSessionsLibrary.MakeLiteralSessionPropertyString` "ServerName" ServerName) (`AdvancedSessionsLibrary.MakeLiteralSessionPropertyString` "ServerLanguage" Language) (`AdvancedSessionsLibrary.MakeLiteralSessionPropertyBool` "UseLan" bUseLAN)) (`GameplayStatics.GetPlayerController` 0) PublicConnections 0 bUseLAN
    (:`OnSuccess`
      (`GameplayStatics.OpenLevelBySoftObjectPtr` "/Game/Maps/DevMap.DevMap" true "listen"))))

(fn `Get Game Instance Ref`
  (returns (GameInstance :type "/Game/Blueprints/MainMenu/MainMenu_Instance Object Reference"))
  (return self))