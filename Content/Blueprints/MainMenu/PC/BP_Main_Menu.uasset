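; Main menu player controller that manages the Main Menu, Create Server and Server Browser screens, showing the main menu on BeginPlay.
; ShowHideWidget runs only for the local controller and routes a widget enum to ShowWidget or HideWidget.
; ShowWidget lazily creates and caches each widget before adding it to the viewport, while HideWidget removes it from its parent, keeping the reference for reuse.
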(event `self.ReceiveBeginPlay`
  (`self.ShowHideWidget` "NewEnumerator0" true))

(event `ShowHideWidget`
  (params (Widget :type "/Game/Blueprints/MainMenu/Enum/E_MainMenuWidget Enum" :default "NewEnumerator0") (Show :type Boolean))
  (if (`self.IsLocalPlayerController`)
    (if Show
      (`self.ShowWidget` Widget)
      (else
        (`self.HideWidget` Widget)))))

(fn `GetPlayerController`
  (returns (PlayerController :type "/Game/Blueprints/MainMenu/PC/BP_Main_Menu Object Reference"))
  (return self))

(fn `HideWidget`
  (params (Widget :type "/Game/Blueprints/MainMenu/Enum/E_MainMenuWidget Enum" :default "NewEnumerator0"))
  (switch `/Game/Blueprints/MainMenu/Enum/E_MainMenuWidget` Widget
    (:`NewEnumerator0`
      (bind _wbp_mainmenu (`self.WBP_MainMenu`)
        (:`then`
          (`Widget.RemoveFromParent` _wbp_mainmenu))
        (:`else`)))
    (:`NewEnumerator1`
      (bind _wbp_createserver (`self.WBP_CreateServer`)
        (:`then`
          (`Widget.RemoveFromParent` _wbp_createserver))
        (:`else`)))
    (:`NewEnumerator2`
      (bind _wbp_serverbrowser (`self.WBP_ServerBrowser`)
        (:`then`
          (`Widget.RemoveFromParent` _wbp_serverbrowser))
        (:`else`)))))

(fn `ShowWidget`
  (params (WIdget :type "/Game/Blueprints/MainMenu/Enum/E_MainMenuWidget Enum" :default "NewEnumerator0"))
  (switch `/Game/Blueprints/MainMenu/Enum/E_MainMenuWidget` WIdget
    (:`NewEnumerator0`
      (`self.WBP_MainMenu`
        (:`then`
          _)
        (:`else`
          (bind _returnvalue (`|CreateWidget` "/Game/UI/MainMenu/WBP_MainMenu.WBP_MainMenu_C"))
          (bind _output_get (set `self.WBP_MainMenu` _returnvalue))))
      (`UserWidget.AddToViewport` _output_get 0))
    (:`NewEnumerator1`
      (`self.WBP_CreateServer`
        (:`then`
          _)
        (:`else`
          (bind _returnvalue_2 (`|CreateWidget` "/Game/UI/MainMenu/WBP_CreateServer.WBP_CreateServer_C"))
          (bind _output_get_2 (set `self.WBP_CreateServer` _returnvalue_2))))
      (`UserWidget.AddToViewport` _output_get_2 0))
    (:`NewEnumerator2`
      (`self.WBP_ServerBrowser`
        (:`then`
          _)
        (:`else`
          (bind _returnvalue_3 (`|CreateWidget` "/Game/UI/MainMenu/WBP_ServerBrowser.WBP_ServerBrowser_C"))
          (bind _output_get_3 (set `self.WBP_ServerBrowser` _returnvalue_3))))
      (`UserWidget.AddToViewport` _output_get_3 0))))

(fn `UserConstructionScript`)